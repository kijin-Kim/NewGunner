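; Death camera pawn for the Gunner that tilts its view down toward a target location, presumably where the player died.
; BeginPlay derives a negative pitch delta from the angle between camera forward and the direction to TargetActorRootLocation.
; While locally viewed, Tick applies that pitch at a constant rate over BlendTime until the remaining angle is used up.
; Pressing 9 spawns a new BP_GunnerPlayerCharacter at the target location and possesses it.
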(event `self.ReceiveBeginPlay`
  (bind _output_get (set `self.StartDeltaPitch` (* (`KismetMathLibrary.RadiansToDegrees` (`KismetMathLibrary.Acos` (`KismetMathLibrary.Dot_VectorVector` (`SceneComponent.GetForwardVector` (`self.Camera`)) (`KismetMathLibrary.Normal` (- (`self.TargetActorRootLocation`) (`self.K2_GetActorLocation`)))))) -1.0)))
  (set `self.RemainedDeltaPitchAbs` (`KismetMathLibrary.Abs` _output_get)))

(event `self.ReceiveTick`
  (params (DeltaSeconds :type "Float (single-precision)"))
  (`parent.ReceiveTick` DeltaSeconds)
  (if (and (> (`self.RemainedDeltaPitchAbs`) 0.0) (`self.IsLocallyViewed`))
    (bind _output_get (set `self.DeltaPitchToAdd` (* (`GameplayStatics.GetWorldDeltaSeconds`) (/ (`self.StartDeltaPitch`) (`self.BlendTime`)))))
    (`SceneComponent.K2_AddLocalRotation` (`self.Camera`) (`KismetMathLibrary.MakeRotator` 0.0 _output_get) false false)
    (set `self.RemainedDeltaPitchAbs` (- (`self.RemainedDeltaPitchAbs`) (`KismetMathLibrary.Abs` (`self.DeltaPitchToAdd`))))))

(event `Key|Nine`
  (params (Key :type "Key Structure"))
  (:`Pressed`
    (bind _returnvalue (`|SpawnActorFromClass` "/Game/Gunner/Characters/_Core/BP_GunnerPlayerCharacter.BP_GunnerPlayerCharacter_C" (`KismetMathLibrary.MakeTransform` (`self.TargetActorRootLocation`)) "Undefined" "MultiplyWithRoot" null null))
    (bind _asplayer_controller (cast `PlayerController` (`self.GetController`)))
    (`Controller.Possess` _asplayer_controller _returnvalue)))

(fn `UserConstructionScript`)