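; BP_GunnerPlayerCharacter is the Gunner player character Blueprint, with a first-person mesh, spring arm and camera.
; Its construction script measures the Root-to-Camera socket distance on the first-person mesh to set that mesh's relative height.
; It also places the spring arm at that distance minus the capsule half-height, so placement follows the skeleton.
; Each tick it draws a short debug line along the camera's forward vector.
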(event `self.ReceiveTick`
  (params (DeltaSeconds :type "Float (single-precision)"))
  (`parent.ReceiveTick` DeltaSeconds)
  (`KismetSystemLibrary.DrawDebugLine` (`SceneComponent.K2_GetComponentLocation` (`self.FirstPersonCameraComponent`)) (+ (`SceneComponent.K2_GetComponentLocation` (`self.FirstPersonCameraComponent`)) (* (`SceneComponent.GetForwardVector` (`self.FirstPersonCameraComponent`)) 300.0)) (struct :`G` 1.0 :`B` 0.003621 :`A` 1.0) 0.0 1.0))

(fn `UserConstructionScript`
  (bind _result (`/Engine/EditorBlueprintResources/StandardMacros.NegateFloat` (`KismetAnimationLibrary.K2_DistanceBetweenTwoSocketsAndMapRange` (`self.FirstPersonMeshComponent`) "Root" "RTS_Component" "Camera" "RTS_Component"))
    (:`  `
      (`SceneComponent.K2_SetRelativeLocation` (`self.FirstPersonMeshComponent`) (`KismetMathLibrary.MakeVector` 0.0 0.0 _result) false true)
      (`SceneComponent.K2_SetRelativeLocation` (`self.FirstPersonSpringArmComponent`) (`KismetMathLibrary.MakeVector` 0.0 0.0 (- (`KismetAnimationLibrary.K2_DistanceBetweenTwoSocketsAndMapRange` (`self.FirstPersonMeshComponent`) "Root" "RTS_Component" "Camera" "RTS_Component") (`CapsuleComponent.GetScaledCapsuleHalfHeight` (`self.CapsuleComponent`)))) false true))))