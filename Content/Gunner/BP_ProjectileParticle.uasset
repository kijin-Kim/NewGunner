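; BP_ProjectileParticle is a gunner projectile that shows a Niagara bullet trail and impact effect.
; On BeginPlay it attaches the trail to its static mesh and starts a timer that destroys it after a short lifetime.
; On Hit it calls the parent handler, spawns a BP_ProjectileHit actor and a physical impact effect aligned to the surface normal, then destroys itself.
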(event `self.ReceiveBeginPlay`
  (`NiagaraFunctionLibrary.SpawnSystemAttached` "/Game/VFX_SciFi_Muzzle_And_Impact_Pack_1/VFX/Presets/Bullet_Trails/NE_VFX_Bullet_Trail_Simple_1.NE_VFX_Bullet_Trail_Simple_1" (`self.StaticMesh`) "None" (0.0 0.0 0.0) (struct) "KeepRelativeOffset" true)
  (`KismetSystemLibrary.K2_SetTimerDelegate` (delegate `DestroySelf`) 2.0))

(event `DestroySelf`
  (`self.K2_DestroyActor`))

(event `self.ReceiveHit`
  (params (MyComp :type "PrimitiveComponent Object Reference") (Other :type "Actor Object Reference") (OtherComp :type "PrimitiveComponent Object Reference") (bSelfMoved :type Boolean) (HitLocation :type "Vector Structure") (HitNormal :type "Vector Structure") (NormalImpulse :type "Vector Structure") (Hit :type "HitResult Structure (by ref)"))
  (bind _returnvalue (`KismetMathLibrary.MakeRotFromX` HitNormal))
  (`parent.ReceiveHit` MyComp Other OtherComp bSelfMoved HitLocation HitNormal NormalImpulse Hit)
  (`|SpawnActorFromClass` "/Game/Gunner/BP_ProjectileHit.BP_ProjectileHit_C" (`KismetMathLibrary.MakeTransform` HitLocation _returnvalue) "Undefined" "MultiplyWithRoot" null null)
  (`NiagaraFunctionLibrary.SpawnSystemAtLocation` "/Game/VFX_SciFi_Muzzle_And_Impact_Pack_1/VFX/Presets/Impacts/NE_VFX_Projectile_Impact_Physical_1.NE_VFX_Projectile_Impact_Physical_1" HitLocation _returnvalue)
  (`self.K2_DestroyActor`))

(fn `UserConstructionScript`)