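; BP_GunnerPlayerCharacter is the Gunner2 player character Blueprint, whose construction script positions its first-person components.
; It first snaps FirstPersonSpringArmComponent to the CameraSocket on FirstPersonMeshComponent.
; It then moves that mesh to the bottom of the capsule, using the scaled half-height as a downward world Z offset.
; Both moves teleport without sweeping, and the socket is read before the mesh moves.
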(fn `UserConstructionScript`
  (`SceneComponent.K2_SetWorldLocation` (`self.FirstPersonSpringArmComponent`) (`SceneComponent.GetSocketLocation` (`self.FirstPersonMeshComponent`) "CameraSocket") false true)
  (`SceneComponent.K2_SetWorldLocation` (`self.FirstPersonMeshComponent`) (- (`SceneComponent.K2_GetComponentLocation` (`self.CapsuleComponent`)) (`KismetMathLibrary.MakeVector` 0.0 0.0 (`CapsuleComponent.GetScaledCapsuleHalfHeight` (`self.CapsuleComponent`)))) false true))